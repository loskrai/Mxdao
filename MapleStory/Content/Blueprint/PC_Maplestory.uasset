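; Player controller for a Maplestory-style game that handles character selection, spawning and possession, and HUD updates.
; On BeginPlay it creates the character select and main UI widgets through a client event, adding only the selection screen to the viewport.
; Selection goes through a server event to the game mode via interface message, while SpawnPlayer spawns and possesses the chosen class.
; Client events forward enemy health and experience updates to the main UI.
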(event `self.ReceiveBeginPlay`
  (`self.InitializeWidgets`))

(event `/Game/Blueprint/Interfaces/INT_PlayerController.InitializeWidgets`
  (`self.CL_InitializeWidgets`))

(event `CL_InitializeWidgets`
  (bind _returnvalue (`|CreateWidget` "/Game/UI/WB_CharacterSelect.WB_CharacterSelect_C"))
  (bind _output_get (set `self.WB_CharacterSelection` _returnvalue))
  (`UserWidget.AddToViewport` _output_get 0)
  (bind _returnvalue_2 (`|CreateWidget` "/Game/UI/WB_MainUI.WB_MainUI_C"))
  (set `self.WB_Main` _returnvalue_2))

(event `/Game/Blueprint/Interfaces/INT_PlayerController.SelectCharacter`
  (params (Player :type "Actor Class Reference") (SpawnLocation :type "Vector Structure"))
  (`self.SRV_SelectCharacter` Player SpawnLocation))

(event `SRV_SelectCharacter`
  (params (Player :type "Actor Class Reference") (SpawnLocation :type "Vector Structure"))
  (bind _gamemode (message `/Game/Blueprint/Interfaces/INT_GameMode.GetGameModeRef` (`GameplayStatics.GetGameMode`)))
  (message `/Game/Blueprint/Interfaces/INT_GameMode.RequestSpawnPlayer` _gamemode self Player SpawnLocation))

(event `/Game/Blueprint/Interfaces/INT_PlayerController.SpawnPlayer`
  (params (Player :type "Actor Class Reference") (SpawnTransform :type "Transform Structure"))
  (bind _returnvalue (`|SpawnActorFromClass` Player SpawnTransform "AdjustIfPossibleButAlwaysSpawn" "MultiplyWithRoot" null null))
  (bind _player (message `/Game/Blueprint/Interfaces/INT_PlayerBase.GetPlayerRef` _returnvalue))
  (`self.Possess` _player))

(event `/Game/Blueprint/Interfaces/INT_PlayerController.UpdateHealthBox`
  (params (Percent :type "Float (double-precision)") (EnemyName :type String))
  (`self.CL_UpdateHealthBox` Percent EnemyName))

(event `CL_UpdateHealthBox`
  (params (Percent :type "Float (single-precision)") (EnemyName :type String))
  (`/Game/UI/WB_MainUI.UpdateHealth` (`self.WB_Main`) Percent EnemyName))

(event `/Game/Blueprint/Interfaces/INT_PlayerController.UpdateEXP`
  (params (PlayerInfo :type "/Game/Blueprint/Structs/ST_PlayerInfo Structure"))
  (`self.CL_UpdateEXP` PlayerInfo))

(event `CL_UpdateEXP`
  (params (PlayerInfo :type "/Game/Blueprint/Structs/ST_PlayerInfo Structure"))
  (`/Game/UI/WB_MainUI.UpdateExperience` (`self.WB_Main`) PlayerInfo))

(fn `GetPlayerControllerRef`
  (returns (PlayerController :type "/Game/Blueprint/PC_Maplestory Object Reference"))
  (return self))

(fn `UserConstructionScript`)