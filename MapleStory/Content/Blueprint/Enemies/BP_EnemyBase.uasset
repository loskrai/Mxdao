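; Base Paper2D flipbook enemy for multiplayer, with contact damage, hit reactions, death and respawn.
; Damage halts AI logic, then survivors repeatedly charge and reposition around the attacker until the player dies and the behavior tree restarts.
; Death awards EXP, fades the sprite, then respawns at a random navmesh point after a delay.
; Overlaps drive a looping damage timer; server events set RepNotify state that updates animation, material, fade color and location.
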(event `/Game/Blueprint/Interfaces/INT_EnemyBase.SetEnemyMovementState`
  (params (MovementState :type "/Game/Blueprint/Enums/E_MovementState Enum" :default "NewEnumerator0"))
  (`self.SRV_SetEnemyMovementState` MovementState))

(event `SRV_SetEnemyMovementState`
  (params (MovementState :type "/Game/Blueprint/Enums/E_MovementState Enum" :default "NewEnumerator0"))
  (set `self.MovementState` MovementState))

(event `self.ReceiveAnyDamage`
  (params (Damage :type "Float (single-precision)") (DamageType :type "DamageType Object Reference") (InstigatedBy :type "Controller Object Reference") (DamageCauser :type "Actor Object Reference"))
  (bind _animalinfo (`self.AnimalInfo`))
  (bind _animalinfo_2 (`self.AnimalInfo`))
  (bind ((`Name_20_1F30E7784800D40EDE240096432099EF` _name) (`EXP_29_E5A2C1754C452C768BBF8A9BEB6156B0` _exp) (`MaxHealth_23_1A32BAA94DC0ED18094FA8970E767B39` _maxhealth) (`Health_14_0820524043DC300231411DA065027EE9` _health)) (break `/Game/Blueprint/Structs/ST_AnimalInfo` _animalinfo))
  (bind _returnvalue (`Controller.K2_GetPawn` (`self.PlayerController`)))
  (bind _x (.x (`self.K2_GetActorLocation`)))
  (set `self.PlayerDamageAmountDamage` Damage)
  (`/Game/Blueprint/Libraries/FunctionLibrary.DisplayFloatingText` self)
  (set `self.PlayerController` InstigatedBy)
  (`/Game/Blueprint/Interfaces/INT_EnemyBase.SetEnemyMovementState` "NewEnumerator7")
  (`CharacterMovementComponent.SetMovementMode` (`self.CharacterMovement`) "MOVE_None" 0)
  (bind _structout (setmembers `/Game/Blueprint/Structs/ST_AnimalInfo` :`StructRef` _animalinfo :`Health` (`KismetMathLibrary.FClamp` (- _health Damage) 0.0 _health)))
  (bind _output_get (set `self.AnimalInfo` _structout))
  (`MovementComponent.StopMovementImmediately` (`self.CharacterMovement`))
  (bind _aicontroller (message `/Game/Blueprint/Interfaces/INT_AIController.GetALControllerRef` (`self.GetController`)))
  (`BrainComponent.StopLogic` (`AIController.BrainComponent` _aicontroller) "Hit")
  (`KismetSystemLibrary.Delay` (`PaperFlipbookComponent.GetFlipbookLength` (`self.Sprite`)))
  (if (== (`.Health_14_0820524043DC300231411DA065027EE9` (break `/Game/Blueprint/Structs/ST_AnimalInfo` _output_get)) 0.0)
    (bind _player (message `/Game/Blueprint/Interfaces/INT_PlayerBase.GetPlayerRef` (`Controller.K2_GetPawn` (`self.PlayerController`))))
    (message `/Game/Blueprint/Interfaces/INT_PlayerBase.AddExperience` _player (`.EXP_29_E5A2C1754C452C768BBF8A9BEB6156B0` (break `/Game/Blueprint/Structs/ST_AnimalInfo` (`self.AnimalInfo`))))
    (`/Game/Blueprint/Interfaces/INT_EnemyBase.Death` true)
    (set `PrimitiveComponent.bGenerateOverlapEvents` false (`self.CapsuleComponent`))
    (set `PrimitiveComponent.bGenerateOverlapEvents` false (`self.Collision`))
    (`/Game/Blueprint/Interfaces/INT_EnemyBase.ActorFade` true)
    (`KismetSystemLibrary.Delay` (`self.RespawnTimer`))
    (bind _structout_2 (setmembers `/Game/Blueprint/Structs/ST_AnimalInfo` :`StructRef` _animalinfo_2 :`Health` (`.MaxHealth_23_1A32BAA94DC0ED18094FA8970E767B39` (break `/Game/Blueprint/Structs/ST_AnimalInfo` _animalinfo_2))))
    (set `self.AnimalInfo` _structout_2)
    (`/Game/Blueprint/Interfaces/INT_EnemyBase.Respawn`)
    (bind _aicontroller_2 (message `/Game/Blueprint/Interfaces/INT_AIController.GetALControllerRef` (`self.GetController`)))
    (`BrainComponent.StartLogic` (`AIController.BrainComponent` _aicontroller_2))
    (set `PrimitiveComponent.bGenerateOverlapEvents` true (`self.CapsuleComponent`))
    (set `PrimitiveComponent.bGenerateOverlapEvents` true (`self.Collision`))
    (`/Game/Blueprint/Interfaces/INT_EnemyBase.ActorFade` false)
    (else
      (`CharacterMovementComponent.SetMovementMode` (`self.CharacterMovement`) "MOVE_Walking" 0)
      (message `/Game/Blueprint/Interfaces/INT_EnemyBase.SetEnemyMovementState` self "NewEnumerator1")
      (`|AIMoveTo` self (`self.K2_GetActorLocation` _returnvalue) _returnvalue 2.0 :!label _label
        (:`OnSuccess`
          (bind _player_2 (message `/Game/Blueprint/Interfaces/INT_PlayerBase.GetPlayerRef` (`Controller.K2_GetPawn` (`self.PlayerController`))))
          (if (not (`/Game/Blueprint/Players/BP_PlayerBase.bIsDead` _player_2))
            (`AITask_MoveTo.AIMoveTo` (`AIBlueprintHelperLibrary.GetAIController` self) (`KismetMathLibrary.MakeVector` (+ _x (`KismetMathLibrary.SelectFloat` -125.0 125.0 (< (.x (`self.K2_GetActorLocation` (`Controller.K2_GetPawn` (`self.PlayerController`)))) _x))) (.y (`self.K2_GetActorLocation`)) (.z (`self.K2_GetActorLocation`))) null
              (:`OnMoveFinished`
                (goto _label)))
            (else
              (`/Game/Blueprint/Interfaces/INT_EnemyBase.RestartBehaviorTree`))))))))

(event `/Game/Blueprint/Interfaces/INT_EnemyBase.StartApplyDamage`
  (params (bApplyDamage :type Boolean))
  (`self.SRV_StartApplyDamage` bApplyDamage))

(event `SRV_StartApplyDamage`
  (params (ApplyDamage :type Boolean))
  (if ApplyDamage
    (bind _returnvalue (`KismetSystemLibrary.K2_SetTimerDelegate` (delegate `ApplyDamage`) 0.1 true))
    (set `self.ApplyDamageHandle` _returnvalue)
    (else
      (`KismetSystemLibrary.K2_ClearAndInvalidateTimerHandle` (`self.ApplyDamageHandle`)))))

(event `/Game/Blueprint/Interfaces/INT_EnemyBase.Respawn`
  (`self.SRV_Respawn`))

(event `ApplyDamage`
  (bind (_animalinfo_name _animalinfo_exp _animalinfo_maxhealth _animalinfo_health _animalinfo_damage) (break `/Game/Blueprint/Structs/ST_AnimalInfo` (`self.AnimalInfo`)))
  (for _array_element (`self.GetOverlappingActors` "/Game/Blueprint/Players/BP_PlayerBase.BP_PlayerBase_C")
    (bind _player (message `/Game/Blueprint/Interfaces/INT_PlayerBase.GetPlayerRef` _array_element))
    (if (not (`/Game/Blueprint/Players/BP_PlayerBase.bGodMode` _player))
      (`GameplayStatics.ApplyDamage` _array_element _animalinfo_damage (`self.GetController`) null "/Script/Engine.DamageType"))))

(event `SRV_Respawn`
  (bind _returnvalue (`GameplayStatics.GetActorOfClass` "/Script/NavigationSystem.NavMeshBoundsVolume"))
  (set `self.SpawnLocation` (`KismetMathLibrary.MakeVector_NetQuantize` (.x (`NavigationSystemV1.K2_GetRandomReachablePointInRadius` (`self.K2_GetActorLocation`) (.x (`.BoxExtent` (`self.GetActorBounds` _returnvalue false false))) null null)) (.y (`self.K2_GetActorLocation`)) (+ (.z (`NavigationSystemV1.K2_GetRandomReachablePointInRadius` (`self.K2_GetActorLocation`) (.x (`.BoxExtent` (`self.GetActorBounds` _returnvalue false false))) null null)) 20.0))))

(event `/Game/Blueprint/Interfaces/INT_EnemyBase.ActorFade`
  (params (bFade :type Boolean))
  (`self.SRV_ActorFade` bFade))

(event `/Game/Blueprint/Interfaces/INT_EnemyBase.RestartBehaviorTree`
  (`self.CL_RestartBehaviorTree`))

(event `CL_RestartBehaviorTree`
  (`MovementComponent.StopMovementImmediately` (`self.CharacterMovement`))
  (`BrainComponent.StopLogic` (`AIController.BrainComponent` (`AIBlueprintHelperLibrary.GetAIController` self)) "")
  (bind _aicontroller (message `/Game/Blueprint/Interfaces/INT_AIController.GetALControllerRef` (`AIBlueprintHelperLibrary.GetAIController` self)))
  (message `/Game/Blueprint/Interfaces/INT_AIController.RunAlTree` _aicontroller))

(event `SRV_ActorFade`
  (params (Fade :type Boolean))
  (bind _output_get (set `self.bActorFade` Fade))
  (if _output_get
    (bind (_direction _fadealpha) (`Timeline|FadingActor` :!via `PlayFromStart` :!label _label_2)
      (:`Update`
        (set `self.ActorFadeColor` (`KismetMathLibrary.LinearColorLerp` (struct :`R` 1.0 :`G` 1.0 :`B` 1.0 :`A` 1.0) (struct :`R` 1.0 :`G` 1.0 :`B` 1.0) _fadealpha)))
      (:`Finished`
        (if (not (`self.bActorFade`))
          (`/Game/Blueprint/Interfaces/INT_EnemyBase.Death` false))))
    (else
      (`CharacterMovementComponent.SetMovementMode` (`self.CharacterMovement`) "MOVE_Walking" 0)
      (goto _label_2 :!via `ReverseFromEnd`))))

(event `self.Collision.OnComponentBeginOverlap`
  (params (OverlappedComponent :type "PrimitiveComponent Object Reference") (OtherActor :type "Actor Object Reference") (OtherComp :type "PrimitiveComponent Object Reference") (OtherBodyIndex :type Integer) (bFromSweep :type Boolean) (SweepResult :type "HitResult Structure (by ref)"))
  (`/Engine/EditorBlueprintResources/ActorMacros.Switch Has Authority`
    (:`Authority`
      (if (`self.ActorHasTag` OtherActor "Player")
        (`/Game/Blueprint/Interfaces/INT_EnemyBase.StartApplyDamage` true)))))

(event `/Game/Blueprint/Interfaces/INT_EnemyBase.Death`
  (params (isDead :type Boolean))
  (`self.SRV_Death` isDead))

(event `self.Collision.OnComponentEndOverlap`
  (params (OverlappedComponent :type "PrimitiveComponent Object Reference") (OtherActor :type "Actor Object Reference") (OtherComp :type "PrimitiveComponent Object Reference") (OtherBodyIndex :type Integer))
  (`/Engine/EditorBlueprintResources/ActorMacros.Switch Has Authority`
    (:`Authority`
      (if (`self.ActorHasTag` OtherActor "Player")
        (`/Game/Blueprint/Interfaces/INT_EnemyBase.StartApplyDamage` false)))))

(event `SRV_Death`
  (params (isDead :type Boolean))
  (bind _output_get (set `self.bIsDead` isDead))
  (if _output_get
    (`self.MC_Death` (`.DeathSFX_26_CF1081CF4A34A96B3036C0B73F9B2F65` (break `/Game/Blueprint/Structs/ST_AnimalInfo` (`self.AnimalInfo`))) (`self.K2_GetActorLocation`))))

(event `MC_Death`
  (params (EnemyDeadSFX :type "SoundBase Object Reference") (Location :type "Vector Structure"))
  (`GameplayStatics.PlaySoundAtLocation` EnemyDeadSFX Location (struct) 1.0 1.0 0.0 null null null null))

(fn `GetEnemyRef`
  (returns (Enemy :type "/Game/Blueprint/Enemies/BP_EnemyBase Object Reference"))
  (return self))

(fn `OnRep_ActorFadeColor`
  (`PaperFlipbookComponent.SetSpriteColor` (`self.Sprite`) (`self.ActorFadeColor`)))

(fn `OnRep_bIsDead`
  (if (`self.bIsDead`)
    (`/Game/Blueprint/Interfaces/INT_EnemyBase.SetEnemyMovementState` "NewEnumerator6")
    (`PrimitiveComponent.SetMaterial` (`self.Sprite`) 0 "/Paper2D/TranslucentUnlitSpriteMaterial.TranslucentUnlitSpriteMaterial")
    (else
      (`PrimitiveComponent.SetMaterial` (`self.Sprite`) 0 "/Paper2D/MaskedUnlitSpriteMaterial.MaskedUnlitSpriteMaterial"))))

(fn `OnRep_bIsMoving`
  (bind (_animalinfo_name _animalinfo_exp _animalinfo_maxhealth _animalinfo_health _animalinfo_damage _animalinfo_idleanimation _animalinfo_moveanimation) (break `/Game/Blueprint/Structs/ST_AnimalInfo` (`self.AnimalInfo`)))
  (bind _sprite (`self.Sprite`))
  (if (not (`self.bIsMoving`))
    (`PaperFlipbookComponent.SetFlipbook` _sprite _animalinfo_idleanimation)
    (else
      (`PaperFlipbookComponent.SetFlipbook` _sprite _animalinfo_moveanimation))))

(fn `OnRep_MovementState`
  (bind _sprite (`self.Sprite`))
  (bind ((`EXP_29_E5A2C1754C452C768BBF8A9BEB6156B0` _exp) (`IdleAnimation_3_69E809934B158340F664DD95AF19EB93` _idleanimation) (`MoveAnimation_5_03CDDBA344C6643BE9E5599D445FE159` _moveanimation) (`HitAnimation_10_7997A2B94D0FADD8EF943D9EEBD525FC` _hitanimation) (`DeathAnimtion_11_68BB49004A80890F6EF3F4B68DBCB59D` _deathanimtion)) (break `/Game/Blueprint/Structs/ST_AnimalInfo` (`self.AnimalInfo`)))
  (switch `/Game/Blueprint/Enums/E_MovementState` (`self.MovementState`)
    (:`NewEnumerator0`
      (`PaperFlipbookComponent.SetFlipbook` _sprite _idleanimation))
    (:`NewEnumerator1`
      (`PaperFlipbookComponent.SetFlipbook` _sprite _moveanimation))
    (:`NewEnumerator6`
      (`PaperFlipbookComponent.SetFlipbook` _sprite _deathanimtion))
    (:`NewEnumerator7`
      (`PaperFlipbookComponent.SetFlipbook` _sprite _hitanimation))))

(fn `OnRep_SpawnLocation`
  (`self.K2_SetActorLocation` (`self.SpawnLocation`)))

(fn `UserConstructionScript`
  (`parent.UserConstructionScript`))