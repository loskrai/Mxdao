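; Base networked 2D flipbook player character for a side-scrolling game, handling movement, jumping, rope and ladder climbing, melee attacks, damage, death/respawn and EXP leveling.
; Actions route through SRV events into state variables, whose OnRep functions apply flipbooks, movement mode, collision and location, while MC events play SFX and VFX.
; PlayerInfo supplies stats and assets, and the controller receives health and EXP updates.
; A separately spawned camera lerps toward a timer-sampled player location.
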(event `MC_AddExperience`
  (params (LevelUpSFX :type "SoundBase Object Reference") (Location :type "Vector Structure") (LevelUp :type "PaperFlipbook Object Reference"))
  (bind _levelupvfx (`self.LevelUpVFX`))
  (`GameplayStatics.PlaySoundAtLocation` LevelUpSFX Location (struct) 1.0 1.0 0.0 null null null null)
  (`SceneComponent.SetVisibility` _levelupvfx true false)
  (`PaperFlipbookComponent.SetFlipbook` _levelupvfx LevelUp)
  (`KismetSystemLibrary.Delay` (`PaperFlipbookComponent.GetFlipbookLength` _levelupvfx))
  (`SceneComponent.SetVisibility` _levelupvfx false false))

(event `/Game/Blueprint/Interfaces/INT_PlayerBase.AddExperience`
  (params (ExperienceToAdd :type Integer))
  (`self.SRV_AddExperience` ExperienceToAdd))

(event `SRV_AddExperience`
  (params (ExperienceToAdd :type Integer))
  (bind _playerinfo (`self.PlayerInfo`))
  (bind ((`EXP_52_4355EE4342D761A24B2F71AF2C982139` _exp)) (break `/Game/Blueprint/Structs/ST_PlayerInfo` _playerinfo))
  (bind _structout (setmembers `/Game/Blueprint/Structs/ST_PlayerInfo` :`StructRef` _playerinfo :`EXP` (+ ExperienceToAdd _exp)))
  (bind _output_get (set `self.PlayerInfo` _structout))
  (bind ((`Level_50_AA4B684A44673C61148EAD8D0EE90EC8` _level) (`EXP_52_4355EE4342D761A24B2F71AF2C982139` _exp_2)) (break `/Game/Blueprint/Structs/ST_PlayerInfo` _output_get))
  (bind ((`EXPrequired_5_F98CCDEF4A72D3DEA580CF9EA398A172` _exprequired)) (break `/Game/Blueprint/Structs/ST_LevelInfo` (`/Game/Blueprint/Libraries/FunctionLibrary.GetLevelInfo` _level)))
  (if (>= _exp _exprequired) :!label _label
    (bind _structout_2 (setmembers `/Game/Blueprint/Structs/ST_PlayerInfo` :`StructRef` (`self.PlayerInfo`) :`Level` (+ _level 1) :`EXP` (- _exp_2 _exprequired)))
    (bind _output_get_2 (set `self.PlayerInfo` _structout_2))
    (bind ((`LevelUpVFX_59_4FAB1625440960B437FA51A61B3F1091` _levelupvfx) (`LevelUpSFX_57_68EF5EB44C153A3F14EA8FB753486D76` _levelupsfx)) (break `/Game/Blueprint/Structs/ST_PlayerInfo` _output_get_2))
    (`self.MC_AddExperience` _levelupsfx (`self.K2_GetActorLocation`) _levelupvfx)
    (goto _label)
    (else
      (bind _playercontroller (message `/Game/Blueprint/Interfaces/INT_PlayerController.GetPlayerControllerRef` (`self.GetController`)))
      (message `/Game/Blueprint/Interfaces/INT_PlayerController.UpdateEXP` _playercontroller (`self.PlayerInfo`)))))

(event `self.ReceiveBeginPlay`
  (bind (_level _exp _health _maxhealth) (break `/Game/Blueprint/Structs/ST_PlayerInfo` (`self.PlayerInfo`)))
  ;[1 1 1 1 70] Movement
  (`/Game/Blueprint/Interfaces/INT_PlayerBase.SetPlayerSpawnLocation`)
  (`KismetSystemLibrary.Delay` 0.05)
  (bind _returnvalue (`|SpawnActorFromClass` "/Game/Blueprint/BP_Camera.BP_Camera_C" (`KismetMathLibrary.MakeTransform` (`self.K2_GetActorLocation`)) "AlwaysSpawn" "MultiplyWithRoot" null null))
  (set `self.PlayerCamera` _returnvalue)
  (bind _playercontroller (message `/Game/Blueprint/Interfaces/INT_PlayerController.GetPlayerControllerRef` (`self.GetController`)))
  (`/Engine/EditorBlueprintResources/StandardMacros.IsValid` _playercontroller
    (:`Is Valid`
      (`PlayerController.SetViewTargetWithBlend` _playercontroller (`self.PlayerCamera`) 0.0 "VTBlend_Linear" 0.0 false)
      ;;[1 1 1] Set up smooth camera following
      (bind _returnvalue_2 (`KismetSystemLibrary.K2_SetTimerDelegate` (delegate `UpdateCameraPosition`) 0.033 true))
      (set `self.UpdateCameraPositionByHandle` _returnvalue_2)
      (bind _returnvalue_3 (`KismetSystemLibrary.K2_SetTimer` null "f_GetCurrentPlayerLocation" 0.1 true))
      (set `self.GetCurrentPlayerLocationHandle` _returnvalue_3)
      (bind _playercontroller_2 (message `/Game/Blueprint/Interfaces/INT_PlayerController.GetPlayerControllerRef` (`self.GetController`)))
      (message `/Game/Blueprint/Interfaces/INT_PlayerController.UpdateHealthBox` _playercontroller_2 (/ _health _maxhealth) "")
      (bind _playercontroller_3 (message `/Game/Blueprint/Interfaces/INT_PlayerController.GetPlayerControllerRef` (`self.GetController`)))
      (message `/Game/Blueprint/Interfaces/INT_PlayerController.UpdateEXP` _playercontroller_3 (`self.PlayerInfo`)))))

(event `UpdateCameraPosition`
  ;[1 1 1 1 70] Movement
  ;;[1 1 1] Set up smooth camera following
  (bind (_direction _movementalpha) (`Timeline|PlayerCameraPosition` :!via `PlayFromStart`)
    (:`Update`
      (`self.K2_SetActorLocation` (`self.PlayerCamera`) (`KismetMathLibrary.VLerp` (`self.K2_GetActorLocation` (`self.PlayerCamera`)) (`self.CurrentPlayerLocation`) _movementalpha) false false))))

(event `/Game/Blueprint/Interfaces/INT_PlayerBase.SetPlayerSpawnLocation`
  ;[1 1 1 1 70] Movement
  ;;[1 1 1] Setting player initial spawn location
  (`self.SRV_SetPlayerSpawnLocation`))

(event `SRV_SetPlayerSpawnLocation`
  ;[1 1 1 1 70] Movement
  ;;[1 1 1] Setting player initial spawn location
  (bind _gamemode (message `/Game/Blueprint/Interfaces/INT_GameMode.GetGameModeRef` (`GameplayStatics.GetGameMode`)))
  (set `self.PlayerSpawnLocation` (`/Game/Blueprint/GM_Maplestory.PlayerSpawnLocation` _gamemode)))

(event `/Game/Blueprint/Interfaces/INT_PlayerBase.PausePlayerCamera`
  (params (Pause :type Boolean))
  ;[1 1 1 1 70] Movement
  ;;[1 1 1] Set up smooth camera following
  (`self.CL_PausePlayerCamera` Pause))

(event `InputAction|Attack`
  (params (Key :type "Key Structure"))
  ;[1 1 1] Attack
  (:`Pressed`
    (if (and (not (`self.BisAttack`)) (not (`self.bIsDead`)) (not (`self.bisClimbing`)))
      (`/Game/Blueprint/Interfaces/INT_PlayerBase.Attack` true))))

(event `MC_Attack`
  (params (AttackSFX :type "SoundBase Object Reference") (Location :type "Vector Structure"))
  ;[1 1 1] Attack
  (`GameplayStatics.PlaySoundAtLocation` AttackSFX Location (struct) 1.0 1.0 0.0 null null null null))

(event `CL_PausePlayerCamera`
  (params (Pause :type Boolean))
  (bind _getcurrentplayerlocationhandle (`self.GetCurrentPlayerLocationHandle`))
  ;[1 1 1 1 70] Movement
  ;;[1 1 1] Set up smooth camera following
  (if Pause
    (`KismetSystemLibrary.K2_PauseTimerHandle` _getcurrentplayerlocationhandle)
    (else
      (`KismetSystemLibrary.K2_UnPauseTimerHandle` _getcurrentplayerlocationhandle))))

(event `/Game/Blueprint/Interfaces/INT_PlayerBase.Attack`
  (params (bisAttack :type Boolean))
  ;[1 1 1] Attack
  (`self.SRV_Attack` bisAttack))

(event `SRV_Attack`
  (params (bisAttack :type Boolean))
  (bind _overlappingactors (`self.GetOverlappingActors` "/Game/Blueprint/Enemies/BP_EnemyBase.BP_EnemyBase_C"))
  ;[1 1 1] Attack
  (set `self.BisAttack` bisAttack)
  (if (!= (`KismetArrayLibrary.Array_Length` _overlappingactors) 0)
    (`self.MC_Attack` (`.AttackHitSFX_42_051BD27144CE8565E65B508E3086C568` (break `/Game/Blueprint/Structs/ST_PlayerInfo` (`self.PlayerInfo`))) (`self.K2_GetActorLocation`))
    (for _array_element _overlappingactors
      (`GameplayStatics.ApplyDamage` _array_element (* (`.BaseDamage_27_0765B94D4625414E870E1B95F6D27D25` (break `/Game/Blueprint/Structs/ST_PlayerInfo` (`self.PlayerInfo`))) (`self.DamageMultiple`)) (`self.GetController`) null "/Script/Engine.DamageType"))
    (else
      (`self.MC_Attack` (`.AttackSFX_40_1283931D4B0496CDD060DDA3D212ABF6` (break `/Game/Blueprint/Structs/ST_PlayerInfo` (`self.PlayerInfo`))) (`self.K2_GetActorLocation`))))
  (`KismetSystemLibrary.Delay` (`PaperFlipbookComponent.GetFlipbookLength` (`self.Sprite`)))
  (set `self.BisAttack` false))

(event `InputAxis|Move_Right/Left`
  (params (AxisValue :type "Float (single-precision)"))
  ;[1 1 1 1 70] Movement
  ;;[1 1 1] PlayerMovement
  (if (and (not (`self.BisAttack`)) (not (`self.bisClimbing`)) (not (`self.bIsDead`)))
    (`self.AddMovementInput` (`KismetMathLibrary.GetForwardVector` (`self.GetControlRotation`)) AxisValue)
    (if (`NavMovementComponent.IsFalling` (`self.CharacterMovement`))
      (if (not (`self.isHitted`))
        (if (> (.z (`self.GetVelocity`)) 0.0)
          (`/Game/Blueprint/Interfaces/INT_PlayerBase.SetMovementState` "NewEnumerator3")
          (else
            (`/Game/Blueprint/Interfaces/INT_PlayerBase.SetMovementState` "NewEnumerator4")))
        (else
          (`/Game/Blueprint/Interfaces/INT_PlayerBase.SetMovementState` "NewEnumerator7")))
      (elif (== AxisValue 0.0)
        (`/Game/Blueprint/Interfaces/INT_PlayerBase.SetMovementState` "NewEnumerator0")
        (elif (> AxisValue 0.0)
          (`/Game/Blueprint/Interfaces/INT_PlayerBase.SetMovementState` "NewEnumerator1")
          (else
            (`/Game/Blueprint/Interfaces/INT_PlayerBase.SetMovementState` "NewEnumerator2")))))))

(event `/Game/Blueprint/Interfaces/INT_PlayerBase.SetIsClimbing`
  (params (bisClimbing :type Boolean))
  ;[1 1 1 1 70] Movement
  ;;[1 1 1] Climb
  ;;;[1 1 1] SetIsClimbing(actually set bIsClimbing[var])
  (`self.SRV_SetIsClimbing` bisClimbing))

(event `/Game/Blueprint/Interfaces/INT_PlayerBase.SetZAxisValue`
  (params (ZAxis :type "Float (double-precision)"))
  ;[1 1 1 1 70] Movement
  ;;[1 1 1] Climb
  ;;;[1 1 1] SetIsZAxis
  (`self.SRV_SetZAxisValue` ZAxis))

(event `/Game/Blueprint/Interfaces/INT_PlayerBase.AdjustClimbingLocation`
  ;[1 1 1 1 70] Movement
  ;;[1 1 1] Climb
  ;;;[1 1 1] AdjustClimbingLocation(actually set the Climbing Location [var])
  (`self.SRV_AdjustClimbingLocation`))

(event `/Game/Blueprint/Interfaces/INT_PlayerBase.SetCanClimbUp`
  (params (CanClimbUp :type Boolean))
  ;[1 1 1 1 70] Movement
  ;;[1 1 1] Climb
  ;;;[1 1 1] SetCanClimbUp(actually set CanClimbUp[var])
  (`self.SRV_SetCanClimbUp` CanClimbUp))

(event `SRV_AdjustClimbingLocation`
  (bind (_returnvalue_x _returnvalue_y _returnvalue_z) (`KismetMathLibrary.BreakVector` (`self.K2_GetActorLocation`)))
  ;[1 1 1 1 70] Movement
  ;;[1 1 1] Climb
  ;;;[1 1 1] AdjustClimbingLocation(actually set the Climbing Location [var])
  (bind _climbingobject (`self.ClimbingObject`)
    (:`then`
      (bind _returnvalue_x_2 (`KismetMathLibrary.BreakVector` (`self.K2_GetActorLocation` _climbingobject)))
      (set `self.ClimbingLocation` (`KismetMathLibrary.MakeVector` _returnvalue_x_2 _returnvalue_y _returnvalue_z)))
    (:`else`)))

(event `SRV_SetIsClimbing`
  (params (isClimbing :type Boolean))
  ;[1 1 1 1 70] Movement
  ;;[1 1 1] Climb
  ;;;[1 1 1] SetIsClimbing(actually set bIsClimbing[var])
  (set `self.bisClimbing` isClimbing))

(event `SRV_SetZAxisValue`
  (params (ZAxis :type "Float (double-precision)"))
  ;[1 1 1 1 70] Movement
  ;;[1 1 1] Climb
  ;;;[1 1 1] SetIsZAxis
  (set `self.ZAxis` ZAxis))

(event `SRV_SetCanClimbUp`
  (params (CanClimbUp :type Boolean))
  ;[1 1 1 1 70] Movement
  ;;[1 1 1] Climb
  ;;;[1 1 1] SetCanClimbUp(actually set CanClimbUp[var])
  (bind _output_get (set `self.CanClimbUp` CanClimbUp))
  (if (and (not _output_get) (`self.bisClimbing`))
    (set `self.CollisionState` "NewEnumerator1")
    (else
      (set `self.CollisionState` "NewEnumerator0"))))

(event `/Game/Blueprint/Interfaces/INT_PlayerBase.PauseClimbFlipbook`
  (params (PauseClimbFlipbook :type Boolean))
  ;[1 1 1 1 70] Movement
  ;;[1 1 1] Climb
  ;;;[1 1 1] SetPauseClimbFlipbook(actually set PauseClimbFlipbookp[var])
  (`self.SRV_PauseClimbFlipbook` PauseClimbFlipbook))

(event `/Game/Blueprint/Interfaces/INT_PlayerBase.SetMovementState`
  (params (MovementState :type "/Game/Blueprint/Enums/E_MovementState Enum" :default "NewEnumerator0"))
  ;[1 1 1 1 70] Movement
  ;;[1 1 1] ChangeMovementState
  (`self.SRV_SetMovementState` MovementState))

(event `/Game/Blueprint/Interfaces/INT_PlayerBase.CanClimb`
  (params (CanClimb :type Boolean) (ClimbingObject :type "PaperSpriteActor Object Reference"))
  ;[1 1 1 1 70] Movement
  ;;[1 1 1] Climb
  (`self.SRV_CanClimb` CanClimb ClimbingObject))

(event `InputAction|Jump`
  (params (Key :type "Key Structure"))
  ;[1 1 1 1 70] Movement
  ;;[1 1 1] PlayerJump
  (:`Pressed`
    (if (and (`self.f_isNotJumping`) (not (`self.bisClimbing`)) (not (`self.bIsDead`)))
      (`self.Jump`)
      (`self.SRV_Jump`))))

(event `SRV_PauseClimbFlipbook`
  (params (PauseClimbFlipbook :type Boolean))
  ;[1 1 1 1 70] Movement
  ;;[1 1 1] Climb
  ;;;[1 1 1] SetPauseClimbFlipbook(actually set PauseClimbFlipbookp[var])
  (set `self.bPauseClimbFlipbook` PauseClimbFlipbook))

(event `SRV_SetMovementState`
  (params (MovementState :type "/Game/Blueprint/Enums/E_MovementState Enum" :default "NewEnumerator0"))
  ;[1 1 1 1 70] Movement
  ;;[1 1 1] ChangeMovementState
  (set `self.MovementState` MovementState))

(event `SRV_CanClimb`
  (params (CanClimb :type Boolean) (ClimbingObject :type "PaperSpriteActor Object Reference"))
  ;[1 1 1 1 70] Movement
  ;;[1 1 1] Climb
  (set `self.ClimbingObject` ClimbingObject)
  (bind _output_get (set `self.bCanClimb` CanClimb))
  (if _output_get
    (bind _returnvalue (`KismetSystemLibrary.K2_SetTimerDelegate` (delegate `ClimbInput`) 0.1 true))
    (set `self.CheckClimbInputHandle` _returnvalue)
    (elif (`self.bisClimbing`)
      (`/Game/Blueprint/Interfaces/INT_PlayerBase.SetIsClimbing` false)
      (set `self.CollisionState` "NewEnumerator0")
      (else
        (`KismetSystemLibrary.K2_ClearAndInvalidateTimerHandle` (`self.CheckClimbInputHandle`))
        (`PaperFlipbookComponent.Play` (`self.Sprite`))))))

(event `SRV_Jump`
  ;[1 1 1 1 70] Movement
  ;;[1 1 1] PlayerJump
  (`self.MC_Jump` (`.JumpSFX_12_B0AF40114A24844C2C76CEB82FA8F7AB` (break `/Game/Blueprint/Structs/ST_PlayerInfo` (`self.PlayerInfo`))) (`self.K2_GetActorLocation`)))

(event `self.ReceiveAnyDamage`
  (params (Damage :type "Float (single-precision)") (DamageType :type "DamageType Object Reference") (InstigatedBy :type "Controller Object Reference") (DamageCauser :type "Actor Object Reference"))
  (bind _playerinfo (`self.PlayerInfo`))
  (bind ((`Level_50_AA4B684A44673C61148EAD8D0EE90EC8` _level) (`EXP_52_4355EE4342D761A24B2F71AF2C982139` _exp) (`Health_30_C59472504682F291A4D596A48E8A33FA` _health)) (break `/Game/Blueprint/Structs/ST_PlayerInfo` _playerinfo))
  (set `self.EnemyDamageAmount` Damage)
  (set `self.EnemyController` InstigatedBy)
  (`/Game/Blueprint/Libraries/FunctionLibrary.DisplayFloatingText` self "NewEnumerator1")
  (if (`self.bisClimbing`)
    (set `self.bCanClimb` false)
    (set `self.bPauseClimbFlipbook` true)
    (set `self.bisClimbing` false))
  (set `self.bGodMode` true)
  (`self.DamageImpause` (`KismetMathLibrary.MakeVector` (`KismetMathLibrary.SelectFloat` -300.0 300.0 (<= (.x (`self.K2_GetActorLocation`)) (.x (`self.K2_GetActorLocation` (`Controller.K2_GetPawn` (`self.EnemyController`)))))) 0.0 300.0))
  (bind _structout (setmembers `/Game/Blueprint/Structs/ST_PlayerInfo` :`StructRef` _playerinfo :`Health` (`KismetMathLibrary.FClamp` (- _health Damage) 0.0 _health)))
  (bind _output_get (set `self.PlayerInfo` _structout))
  (bind _playercontroller (message `/Game/Blueprint/Interfaces/INT_PlayerController.GetPlayerControllerRef` (`self.GetController`)))
  (bind _enemy (message `/Game/Blueprint/Interfaces/INT_EnemyBase.GetEnemyRef` (`Controller.K2_GetPawn` (`self.EnemyController`))))
  (bind ((`Level_50_AA4B684A44673C61148EAD8D0EE90EC8` _level_2) (`EXP_52_4355EE4342D761A24B2F71AF2C982139` _exp_2) (`Health_30_C59472504682F291A4D596A48E8A33FA` _health_2) (`MaxHealth_34_0D52F6FC42510BBD2B93959E4856DE23` _maxhealth)) (break `/Game/Blueprint/Structs/ST_PlayerInfo` _output_get))
  (message `/Game/Blueprint/Interfaces/INT_PlayerController.UpdateHealthBox` _playercontroller (/ _health_2 _maxhealth) (`.Name_20_1F30E7784800D40EDE240096432099EF` (break `/Game/Blueprint/Structs/ST_AnimalInfo` (`/Game/Blueprint/Enemies/BP_EnemyBase.AnimalInfo` _enemy))))
  (if (== _health_2 0.0)
    (`self.Death` true)
    (else
      (`/Game/Blueprint/Interfaces/INT_PlayerBase.DamageVFX` "/Paper2D/TranslucentUnlitSpriteMaterial.TranslucentUnlitSpriteMaterial" (struct :`R` 1.0 :`G` 1.0 :`B` 1.0 :`A` 0.6))
      (`KismetSystemLibrary.Delay` (`self.GodModeTime`))
      (set `self.bGodMode` false))))

(event `ClimbInput`
  (bind _zaxis (`self.ZAxis`))
  ;[1 1 1 1 70] Movement
  ;;[1 1 1] Climb
  (if (or (< _zaxis 0.0) (and (> _zaxis 0.0) (`self.CanClimbUp`)))
    (`KismetSystemLibrary.K2_ClearAndInvalidateTimerHandle` (`self.CheckClimbInputHandle`))
    (`/Game/Blueprint/Interfaces/INT_PlayerBase.SetIsClimbing` true)
    (set `self.CollisionState` "NewEnumerator1")))

(event `MC_Jump`
  (params (Jump_SFX :type "SoundBase Object Reference") (Player_Location :type "Vector Structure"))
  ;[1 1 1 1 70] Movement
  ;;[1 1 1] PlayerJump
  (`GameplayStatics.PlaySoundAtLocation` Jump_SFX Player_Location (struct) 1.0 1.0 0.0 null null null null))

(event `InputAxis|Move_Up/Down`
  (params (AxisValue :type "Float (single-precision)"))
  (bind _returnvalue_x (`KismetMathLibrary.BreakVector` (`self.K2_GetActorLocation`)))
  ;[1 1 1 1 70] Movement
  ;;[1 1 1] Climb
  (if (and (`self.bCanClimb`) (not (`self.bIsDead`)))
    (`/Game/Blueprint/Interfaces/INT_PlayerBase.SetZAxisValue` AxisValue)
    (`self.AddMovementInput` (`KismetMathLibrary.GetUpVector` (`self.GetControlRotation`)) AxisValue)
    (if (`self.bisClimbing`)
      (if (and (!= (`self.ZAxis`) 0.0) (not (`PaperFlipbookComponent.IsPlaying` (`self.Sprite`))))
        (`/Game/Blueprint/Interfaces/INT_PlayerBase.PauseClimbFlipbook` false)
        (elif (and (== (`self.ZAxis`) 0.0) (`PaperFlipbookComponent.IsPlaying` (`self.Sprite`)))
          (`/Game/Blueprint/Interfaces/INT_PlayerBase.PauseClimbFlipbook` true)
          (else
            (bind _climbingobject (`self.ClimbingObject`)
              (:`then`
                (bind _returnvalue_x_2 (`KismetMathLibrary.BreakVector` (`self.K2_GetActorLocation` _climbingobject)))
                (if (!= _returnvalue_x_2 _returnvalue_x)
                  (`self.AdjustClimbingLocation`)))
              (:`else`))))))))

(event `/Game/Blueprint/Interfaces/INT_PlayerBase.DamageVFX`
  (params (PlayerMaterial :type "MaterialInterface Object Reference") (PlayerColor :type "LinearColor Structure"))
  ;[1 1 1] DamageVFX
  (`self.SRV_DamageVFX` PlayerMaterial PlayerColor))

(event `/Game/Blueprint/Interfaces/INT_PlayerBase.DamageImpause`
  (params (Impause :type "Vector Structure"))
  ;[1 1 1] DamageVFX
  (`self.SRV_DamageImpause` Impause))

(event `MC_DamageImpause`
  (params (Impulse :type "Vector Structure"))
  ;[1 1 1] DamageVFX
  (`CharacterMovementComponent.AddImpulse` (`self.CharacterMovement`) Impulse true))

(event `SRV_DamageVFX`
  (params (Material :type "MaterialInterface Object Reference") (Color :type "LinearColor Structure"))
  ;[1 1 1] DamageVFX
  (`self.MC_DamageVFX` Material Color))

(event `SRV_DamageImpause`
  (params (Impulse :type "Vector Structure"))
  ;[1 1 1] DamageVFX
  (`self.MC_DamageImpause` Impulse))

(event `MC_DamageVFX`
  (params (Material :type "MaterialInterface Object Reference") (Color :type "LinearColor Structure"))
  ;[1 1 1] DamageVFX
  (set `self.isHitted` true)
  (bind _returnvalue (`KismetSystemLibrary.K2_SetTimerDelegate` (delegate `DamegVFXLoop`) (/ (`self.GodModeTime`) 8.0) true))
  (set `self.DamageVFXHandle` _returnvalue)
  (`KismetSystemLibrary.K2_SetTimerDelegate` (delegate `StopDamageVFX`) (`self.GodModeTime`)))

(event `DamegVFXLoop`
  ;[1 1 1] DamageVFX
  (`PrimitiveComponent.SetMaterial` (`self.Sprite`) 0 (stale `MC_DamageVFX` Material))
  (`PaperFlipbookComponent.SetSpriteColor` (`self.Sprite`) (stale `MC_DamageVFX` Color))
  (`KismetSystemLibrary.Delay` (/ (`self.GodModeTime`) 10.0))
  (`PrimitiveComponent.SetMaterial` (`self.Sprite`) 0 "/Paper2D/MaskedUnlitSpriteMaterial.MaskedUnlitSpriteMaterial")
  (`PaperFlipbookComponent.SetSpriteColor` (`self.Sprite`) (struct :`R` 1.0 :`G` 1.0 :`B` 1.0 :`A` 1.0)))

(event `StopDamageVFX`
  ;[1 1 1] DamageVFX
  (set `self.isHitted` false)
  (`KismetSystemLibrary.K2_ClearAndInvalidateTimerHandle` (`self.DamageVFXHandle`)))

(event `/Game/Blueprint/Interfaces/INT_PlayerBase.Death`
  (params (bisDeath :type Boolean))
  (`self.SRV_Death` bisDeath))

(event `SRV_Death`
  (params (isDead :type Boolean))
  (bind _playerinfo (`self.PlayerInfo`))
  (bind ((`Level_50_AA4B684A44673C61148EAD8D0EE90EC8` _level) (`EXP_52_4355EE4342D761A24B2F71AF2C982139` _exp) (`MaxHealth_34_0D52F6FC42510BBD2B93959E4856DE23` _maxhealth) (`LevelUpVFX_59_4FAB1625440960B437FA51A61B3F1091` _levelupvfx) (`DeathSFX_45_D9362FCE41BAD4DDD5D733985401DE8A` _deathsfx) (`RespawnSFX_47_2E4731A14652718FF59CD3B524E8182B` _respawnsfx)) (break `/Game/Blueprint/Structs/ST_PlayerInfo` _playerinfo))
  (`MovementComponent.StopMovementImmediately` (`self.CharacterMovement`))
  (bind _output_get (set `self.bIsDead` isDead))
  (if _output_get
    (`self.MC_Death` _deathsfx (`self.K2_GetActorLocation`))
    (else
      (`self.MC_Death` _respawnsfx (`self.K2_GetActorLocation`))
      (bind _structout (setmembers `/Game/Blueprint/Structs/ST_PlayerInfo` :`StructRef` _playerinfo :`Health` _maxhealth))
      (bind _output_get_2 (set `self.PlayerInfo` _structout))
      (bind _playercontroller (message `/Game/Blueprint/Interfaces/INT_PlayerController.GetPlayerControllerRef` (`self.GetController`)))
      (bind (_level_2 _exp_2 _health _maxhealth_2) (break `/Game/Blueprint/Structs/ST_PlayerInfo` _output_get_2))
      (message `/Game/Blueprint/Interfaces/INT_PlayerController.UpdateHealthBox` _playercontroller (/ _health _maxhealth_2) "")
      (`self.SetPlayerSpawnLocation`)
      (`/Game/Blueprint/Interfaces/INT_PlayerBase.DamageVFX` "/Paper2D/TranslucentUnlitSpriteMaterial.TranslucentUnlitSpriteMaterial" (struct :`R` 1.0 :`G` 1.0 :`B` 1.0 :`A` 0.6))
      (`KismetSystemLibrary.Delay` (`self.GodModeTime`))
      (set `self.bGodMode` false))))

(event `MC_Death`
  (params (EnemyDeadSFX :type "SoundBase Object Reference") (Location :type "Vector Structure"))
  (`GameplayStatics.PlaySoundAtLocation` EnemyDeadSFX Location (struct) 1.0 1.0 0.0 null null null null))

(fn `f_GetCurrentPlayerLocation`
  (set `self.CurrentPlayerLocation` (`self.K2_GetActorLocation`)))

(fn `f_isNotJumping`
  (returns (ReturnValue :type Boolean))
  (return (not (`NavMovementComponent.IsFalling` (`self.CharacterMovement`)))))

(fn `GetPlayerRef`
  (returns (Player :type "/Game/Blueprint/Players/BP_PlayerBase Object Reference"))
  (return self))

(fn `OnRep_bCanClimb`)

(fn `OnRep_BisAttack`
  (if (not (`self.bIsDead`))
    (if (`self.BisAttack`)
      (`self.SetMovementState` "NewEnumerator5")
      (else
        (`self.SetMovementState` "NewEnumerator0")))))

(fn `OnRep_bisClimbing`
  (bind ((`Level_50_AA4B684A44673C61148EAD8D0EE90EC8` _level) (`EXP_52_4355EE4342D761A24B2F71AF2C982139` _exp) (`FallAnimation_9_F80682244D5F7154F293D0A7EE69DB5C` _fallanimation) (`RopeAnimation_15_D873CB3E437D5DA5A033D8819F2D7ED0` _ropeanimation) (`LadderAnimation_18_D95DA18942F923798C9870868378FE5A` _ladderanimation)) (break `/Game/Blueprint/Structs/ST_PlayerInfo` (`self.PlayerInfo`)))
  (if (not (`self.bIsDead`))
    (if (`self.bisClimbing`)
      (`CharacterMovementComponent.SetMovementMode` (`self.CharacterMovement`) "MOVE_Flying" 0)
      (bind _asbp_climbing_base (cast `/Game/Blueprint/Climbing/BP_ClimbingBase` (`self.ClimbingObject`)))
      (switch `/Game/Blueprint/Enums/E_ClimbType` (`/Game/Blueprint/Climbing/BP_ClimbingBase.ClimbingObjectType` _asbp_climbing_base)
        (:`NewEnumerator0`
          (`PaperFlipbookComponent.SetFlipbook` (`self.Sprite`) _ropeanimation))
        (:`NewEnumerator1`
          (`PaperFlipbookComponent.SetFlipbook` (`self.Sprite`) _ladderanimation)))
      (else
        (`CharacterMovementComponent.SetMovementMode` (`self.CharacterMovement`) "MOVE_Falling" 0)
        (`PaperFlipbookComponent.SetFlipbook` (`self.Sprite`) _fallanimation)))
    (else
      (`CharacterMovementComponent.SetMovementMode` (`self.CharacterMovement`) "MOVE_Walking" 0)
      (`/Game/Blueprint/Interfaces/INT_PlayerBase.SetMovementState` "NewEnumerator6"))))

(fn `OnRep_bIsDead`
  (if (`self.bIsDead`)
    (`/Game/Blueprint/Interfaces/INT_PlayerBase.SetMovementState` "NewEnumerator6")))

(fn `OnRep_bPauseClimbFlipbook`
  (bind _sprite (`self.Sprite`))
  (if (`self.bPauseClimbFlipbook`)
    (`PaperFlipbookComponent.Stop` _sprite)
    (else
      (`PaperFlipbookComponent.Play` _sprite))))

(fn `OnRep_ClimbingLocation`
  (`self.K2_SetActorLocation` (`self.ClimbingLocation`)))

(fn `OnRep_ClimbingObject`)

(fn `OnRep_CollisionState`
  (bind _capsulecomponent (`self.CapsuleComponent`))
  (switch `/Game/Blueprint/Enums/E_CollisionState` (`self.CollisionState`)
    (:`NewEnumerator0`
      (`PrimitiveComponent.SetCollisionObjectType` _capsulecomponent "ECC_Pawn"))
    (:`NewEnumerator1`
      (`PrimitiveComponent.SetCollisionObjectType` _capsulecomponent "ECC_GameTraceChannel1"))))

(fn `OnRep_MovementState`
  (bind _sprite (`self.Sprite`))
  (bind (_level _exp _health _maxhealth _basedamage _idelanimation _runanimation _jumpanimation _fallanimation _ropeanimation _ladderanimation _attackanimation _deadanimation _hitanimation) (break `/Game/Blueprint/Structs/ST_PlayerInfo` (`self.PlayerInfo`)))
  (if (not (`self.bisClimbing`))
    (switch `/Game/Blueprint/Enums/E_MovementState` (`self.MovementState`)
      (:`NewEnumerator0`
        (`PaperFlipbookComponent.SetFlipbook` _sprite _idelanimation))
      (:`NewEnumerator1`
        (`SceneComponent.K2_SetRelativeRotation` :`self` _sprite)
        (`PaperFlipbookComponent.SetFlipbook` _sprite _runanimation))
      (:`NewEnumerator2`
        (`SceneComponent.K2_SetRelativeRotation` _sprite (struct :`Yaw` 180.0) false false)
        (`PaperFlipbookComponent.SetFlipbook` _sprite _runanimation))
      (:`NewEnumerator3`
        (`PaperFlipbookComponent.SetFlipbook` _sprite _jumpanimation))
      (:`NewEnumerator4`
        (`PaperFlipbookComponent.SetFlipbook` _sprite _fallanimation))
      (:`NewEnumerator5`
        (`PaperFlipbookComponent.SetFlipbook` _sprite _attackanimation))
      (:`NewEnumerator6`
        (`PaperFlipbookComponent.SetFlipbook` _sprite _deadanimation))
      (:`NewEnumerator7`
        (`PaperFlipbookComponent.SetFlipbook` _sprite _hitanimation)))))

(fn `OnRep_PlayerSpawnLocation`
  (`self.K2_SetActorLocation` (`self.PlayerSpawnLocation`)))

(fn `OnRep_ZAxis`)

(fn `UserConstructionScript`
  (`parent.UserConstructionScript`))